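; One-shot trigger actor that reveals rope skeletal meshes when an actor with "Sphere" in its name overlaps it.
; It finds all actors tagged SkeletalRope, makes their skeletal meshes visible and sets them to block the Pawn channel.
; The Trigger component's drop and the IsTriggerred latch sit inside that loop, so the trigger lowers once per rope processed.
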(event `self.ReceiveActorBeginOverlap`
  (params (OtherActor :type "Actor Object Reference"))
  (bind _trigger (`self.Trigger`))
  (if (`KismetStringLibrary.Contains` (`KismetSystemLibrary.GetObjectName` OtherActor) "Sphere")
    (if (not (`self.IsTriggerred`))
      (bind _outactors (`GameplayStatics.GetAllActorsWithTag` "SkeletalRope"))
      (for _array_element _outactors
        (bind _asskeletal_mesh_actor (cast `SkeletalMeshActor` _array_element))
        (bind _skeletalmeshcomponent (`SkeletalMeshActor.SkeletalMeshComponent` _asskeletal_mesh_actor))
        (`SceneComponent.SetVisibility` _skeletalmeshcomponent true false)
        (`PrimitiveComponent.SetCollisionResponseToChannel` _skeletalmeshcomponent "ECC_Pawn" "ECR_Block")
        (`SceneComponent.K2_SetWorldLocation` _trigger (`KismetMathLibrary.MakeVector` (.x (`SceneComponent.K2_GetComponentLocation` _trigger)) (.y (`SceneComponent.K2_GetComponentLocation` _trigger)) (- (.z (`SceneComponent.K2_GetComponentLocation` _trigger)) 10.0)) false false)
        (set `self.IsTriggerred` true)))))

(fn `UserConstructionScript`)