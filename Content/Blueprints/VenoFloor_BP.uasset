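; VenoFloor_BP is a hazard floor actor that kills the side-scroller character when it overlaps.
; After a short delay it ragdolls the character's mesh by simulating physics on all bodies and disables movement.
; A second delay later it sets the character's Dead flag and moves the first KillZVolume in the level onto the character's location, rather than moving the character to the volume.
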(event `self.ReceiveActorBeginOverlap`
  (params (OtherActor :type "Actor Object Reference"))
  (bind _character (`self.Character`))
  (`KismetSystemLibrary.Delay` 0.2)
  (bind _asside_scroller_character (cast `/Game/SideScrollerCPP/Blueprints/SideScrollerCharacter` OtherActor))
  (set `self.Character` _asside_scroller_character)
  (`SkeletalMeshComponent.SetAllBodiesSimulatePhysics` (`Character.Mesh` _asside_scroller_character) true)
  (bind _ascharacter_movement_component (cast `CharacterMovementComponent` (`Pawn.GetMovementComponent` _asside_scroller_character)))
  (`CharacterMovementComponent.DisableMovement` _ascharacter_movement_component)
  (`KismetSystemLibrary.Delay` 1.0)
  (set `/Game/SideScrollerCPP/Blueprints/SideScrollerCharacter.Dead` true _character)
  (bind _outactors (`GameplayStatics.GetAllActorsOfClass` "/Script/Engine.KillZVolume"))
  (`self.K2_SetActorLocation` (`|GetArrayItem` _outactors) (`SceneComponent.K2_GetComponentLocation` (`Actor.RootComponent` _character)) false false))

(fn `UserConstructionScript`)