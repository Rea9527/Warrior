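; FanTrigger_BP is a one-shot trigger that stops a fan in the level.
; On BeginPlay it caches the first Fan_BP actor it finds.
; When an actor with "Sphere" in its name first overlaps it, it zeroes the fan's RotatingMovement rate, clears the fan's IsTriggerred flag and lowers its own Trigger component like a pressed switch.
; Its own IsTriggerred flag blocks repeat activation.
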(event `self.ReceiveBeginPlay`
  (bind _outactors (`GameplayStatics.GetAllActorsOfClass` "/Game/Blueprints/Fan_BP.Fan_BP_C"))
  (set `self.Fan` (`|GetArrayItem` _outactors)))

(event `self.ReceiveActorBeginOverlap`
  (params (OtherActor :type "Actor Object Reference"))
  (bind _fan (`self.Fan`))
  (if (`KismetStringLibrary.Contains` (`KismetSystemLibrary.GetObjectName` OtherActor) "Sphere")
    (if (not (`self.IsTriggerred`))
      (set `RotatingMovementComponent.RotationRate` (struct) (`/Game/Blueprints/Fan_BP.RotatingMovement` _fan))
      (set `/Game/Blueprints/Fan_BP.IsTriggerred` false _fan)
      (`SceneComponent.K2_SetWorldLocation` (`self.Trigger`) (`KismetMathLibrary.MakeVector` (.x (`SceneComponent.K2_GetComponentLocation` (`self.Trigger`))) (.y (`SceneComponent.K2_GetComponentLocation` (`self.Trigger`))) (- (.z (`SceneComponent.K2_GetComponentLocation` (`self.Trigger`))) 10.0)) false false)
      (set `self.IsTriggerred` true))))

(fn `UserConstructionScript`)