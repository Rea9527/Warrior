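; SphereBox_BP is a trigger actor that releases a Ceiling piece and a Cable when its collision box is overlapped.
; On BeginPlay it binds the overlap and caches the SideScrollerCharacter tagged MainCharacter.
; Overlap enables Ceiling physics, detaches both Cable ends and makes Sphere and character capsule ignore the Destructible channel.
; After a one-second delay it destroys the Ceiling and restores blocking on the capsule only.
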(event `self.ReceiveBeginPlay`
  (add `PrimitiveComponent.OnComponentBeginOverlap` (`self.CollisionComp`) (delegate `CharaBoxOverlap`))
  (bind _outactors (`GameplayStatics.GetAllActorsWithTag` "MainCharacter"))
  (bind _asside_scroller_character (cast `/Game/SideScrollerCPP/Blueprints/SideScrollerCharacter` (`|GetArrayItem` _outactors)))
  (set `self.Character` _asside_scroller_character))

(event `CharaBoxOverlap`
  (params (OverlappedComponent :type "PrimitiveComponent Object Reference") (OtherActor :type "Actor Object Reference") (OtherComp :type "PrimitiveComponent Object Reference") (OtherBodyIndex :type Integer) (bFromSweep :type Boolean) (SweepResult :type "HitResult Structure (by ref)"))
  (bind _cable (`self.Cable`))
  (`PrimitiveComponent.SetSimulatePhysics` (`self.Ceiling`) true)
  (`PrimitiveComponent.SetCollisionResponseToChannel` (`Character.CapsuleComponent` (`self.Character`)) "ECC_Destructible" "ECR_Ignore")
  (`PrimitiveComponent.SetCollisionResponseToChannel` (`self.Sphere`) "ECC_Destructible" "ECR_Ignore")
  (set `CableComponent.bAttachEnd` false _cable)
  (set `CableComponent.bAttachStart` false _cable)
  (`KismetSystemLibrary.Delay` 1.0)
  (`ActorComponent.K2_DestroyComponent` (`self.Ceiling`))
  (`PrimitiveComponent.SetCollisionResponseToChannel` (`Character.CapsuleComponent` (`self.Character`)) "ECC_Destructible" "ECR_Block"))

(fn `UserConstructionScript`)