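; ConveyerTrigger_BP is a one-shot trigger that activates a conveyer when an actor overlaps it.
; On BeginPlay it finds the first actor tagged "Conveyer" and caches it as a Conveyer_BP reference.
; The first overlap sets the conveyer's IsTriggered flag, latches its own flag to block repeats, and lowers the Trigger component slightly, like a pressed switch.
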(event `self.ReceiveBeginPlay`
  (bind _outactors (`GameplayStatics.GetAllActorsWithTag` "Conveyer"))
  (bind _asconveyer_bp (cast `/Game/Blueprints/Conveyer_BP` (`|GetArrayItem` _outactors)))
  (set `self.Conveyer` _asconveyer_bp))

(event `self.ReceiveActorBeginOverlap`
  (params (OtherActor :type "Actor Object Reference"))
  (if (not (`self.IsTriggerred`))
    (set `/Game/Blueprints/Conveyer_BP.IsTriggered` true (`self.Conveyer`))
    (set `self.IsTriggerred` true)
    (`SceneComponent.K2_SetWorldLocation` (`self.Trigger`) (`KismetMathLibrary.MakeVector` (.x (`SceneComponent.K2_GetComponentLocation` (`self.Trigger`))) (.y (`SceneComponent.K2_GetComponentLocation` (`self.Trigger`))) (- (.z (`SceneComponent.K2_GetComponentLocation` (`self.Trigger`))) 10.0)) false false)))

(fn `UserConstructionScript`)