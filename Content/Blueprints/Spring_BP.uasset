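; Spring launch pad that bounces the side-scroller player character straight up.
; Each tick it reads the Spring constraint's linear force, and a positive Z starts a short delay before checking the character's position against hardcoded world Y and height bounds.
; A character inside those bounds gets an upward velocity-change impulse, and a Touched flag blocks retriggering for a second.
; The character is found by the MainCharacter tag at BeginPlay.
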(event `self.ReceiveBeginPlay`
  ;[1 1 1] Get Character
  (bind _outactors (`GameplayStatics.GetAllActorsWithTag` "MainCharacter"))
  (bind _asside_scroller_character (cast `/Game/SideScrollerCPP/Blueprints/SideScrollerCharacter` (`|GetArrayItem` _outactors)))
  (set `self.Character` _asside_scroller_character))

(event `self.ReceiveTick`
  (params (DeltaSeconds :type "Float (single-precision)"))
  (bind _character (`self.Character`))
  (if (not (`self.Touched`))
    (bind _outlinearforce (`PhysicsConstraintComponent.GetConstraintForce` (`self.Spring`)))
    (if (> (.z _outlinearforce) 0.0)
      (`KismetSystemLibrary.Delay` 0.3)
      (if (and (`KismetMathLibrary.InRange_FloatFloat` (.y (`self.K2_GetActorLocation` _character)) 3500.0 3635.0) (>= (.z (`self.K2_GetActorLocation` _character)) 480.0))
        (bind _ascharacter_movement_component (cast `CharacterMovementComponent` (`Pawn.GetMovementComponent` _character)))
        (`CharacterMovementComponent.AddImpulse` _ascharacter_movement_component (0.0 0.0 1700.0) true)
        (set `self.Touched` true)
        (`KismetSystemLibrary.Delay` 1.0)
        (set `self.Touched` false)))))

(fn `UserConstructionScript`)