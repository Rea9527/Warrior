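; Fan Blueprint that pushes the side-scroller character along negative Y, like a wind gust.
; On BeginPlay it caches the first actor tagged MainCharacter.
; While IsTriggerred is set, Tick checks whether the character is inside a hard-coded world-space Y band above a minimum height, then applies a mass-independent velocity impulse through its movement component every frame.
; Nothing in this file sets the trigger flag.
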(event `self.ReceiveBeginPlay`
  (bind _outactors (`GameplayStatics.GetAllActorsWithTag` "MainCharacter"))
  (bind _asside_scroller_character (cast `/Game/SideScrollerCPP/Blueprints/SideScrollerCharacter` (`|GetArrayItem` _outactors)))
  (set `self.Character` _asside_scroller_character))

(event `self.ReceiveTick`
  (params (DeltaSeconds :type "Float (single-precision)"))
  (bind _y (.y (`self.K2_GetActorLocation` (`self.Character`))))
  (if (`self.IsTriggerred`)
    (if (and (> _y 3590.0) (<= _y 3640.0) (>= (.z (`self.K2_GetActorLocation` (`self.Character`))) 2610.0))
      (bind _ascharacter_movement_component (cast `CharacterMovementComponent` (`Pawn.GetMovementComponent` (`self.Character`))))
      (`CharacterMovementComponent.AddImpulse` _ascharacter_movement_component (0.0 -50.0 0.0) true))))

(fn `UserConstructionScript`)