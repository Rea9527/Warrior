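; Side-scroller conveyor belt that carries overlapping characters along and pushes them when they leave.
; Each tick it offsets characters in Box1 and, when triggered, tagged belt meshes by GetDeltaLocation.
; On end overlap it applies a Speed-scaled Y impulse and resets the capsule radius.
; Construction zeroes rotation; the belt wrap from MinY to MaxY is disconnected, and the helper functions' calculations are unused.
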(event `self.ReceiveBeginPlay`
  (bind (_miny _maxy) (`self.GetConveyerMinMaxY`))
  ;[1 1 1] Get Min and Max Y
  (set `self.MinY` _miny)
  (set `self.MaxY` _maxy))

(event `self.ReceiveTick`
  (params (DeltaSeconds :type "Float (single-precision)"))
  (set `self.DeltaTime` DeltaSeconds)
  (`|ExecutionSequence`
    (:`then_0`
      ;[1 1 1] Offset object on conveyer
      (for _array_element (`PrimitiveComponent.GetOverlappingActors` (`self.Box1`) "/Game/SideScrollerCPP/Blueprints/SideScrollerCharacter.SideScrollerCharacter_C")
        (`self.K2_AddActorWorldOffset` _array_element (`self.GetDeltaLocation`) false false)))
    (:`then_1`
      ;[1 1 1] Update belts
      (if (`self.IsTriggered`)
        (for _array_element_2 (`self.GetComponentsByTag` "/Script/Engine.StaticMeshComponent" (`self.BeltsTag`))
          (`SceneComponent.K2_AddWorldOffset` _array_element_2 (`self.GetDeltaLocation`) false false))))))

(event `self.ReceiveActorEndOverlap`
  (params (OtherActor :type "Actor Object Reference"))
  ;[1 1 1] End Overlap - add impulse
  (bind _asside_scroller_character (cast `/Game/SideScrollerCPP/Blueprints/SideScrollerCharacter` OtherActor))
  (bind _ascharacter_movement_component (cast `CharacterMovementComponent` (`Pawn.GetMovementComponent` _asside_scroller_character)))
  (`CharacterMovementComponent.AddImpulse` _ascharacter_movement_component (`KismetMathLibrary.MakeVector` 0.0 (- 0.0 (* (`self.Speed`) 100.0))) false)
  (`CapsuleComponent.SetCapsuleRadius` (`Character.CapsuleComponent` _asside_scroller_character) 34.0 true))

(fn `UserConstructionScript`
  (`self.K2_SetActorRotation` (struct)))